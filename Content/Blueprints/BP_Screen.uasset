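; BP_Screen is a sprite-based screen actor that displays game states such as start, ready, idle, player lights, timer over and game over.
; Events swap sprites on its RenderComponent, using short delays for start and ready animations and per-player arrays for highlights and game-over screens.
; A player press lights that player's sprite, then a retriggerable delay restores idle if BP_GameMode's round has started.
; The ready sequence also triggers the BP_Pattern actor found at BeginPlay.
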(event `Set Background Sprite`
  (params (Sprite :type "PaperSprite Object Reference"))
  ;[1 1 1] Set Background
  (`PaperSpriteComponent.SetSprite` (`self.RenderComponent`) Sprite))

(event `Set Screen Lights Off`
  ;[1 1 1] Turn Off Screen Lights
  (`self.Set Background Sprite` "/Game/Sprites/0_Sprite.0_Sprite"))

(event `Game Over Screen`
  ;[1 1 1] Show Game Over Background
  (`self.Set Background Sprite` "/Game/Sprites/24_Sprite.24_Sprite")
  (`KismetSystemLibrary.Delay` 0.2))

(event `self.ReceiveBeginPlay`
  ;[1 1 1] Init Objects and Sprite Arrays
  (bind _outactors (`GameplayStatics.GetAllActorsOfClass` "/Game/Blueprints/BP_Pattern.BP_Pattern_C"))
  (set `self.Pattern Screen` (`KismetArrayLibrary.Array_Get` _outactors))
  (set `self.Player Screens` (`|MakeArray` "/Game/Sprites/14_Sprite.14_Sprite" "/Game/Sprites/6_Sprite.6_Sprite" "/Game/Sprites/5_Sprite.5_Sprite" "/Game/Sprites/4_Sprite.4_Sprite" :!type "PaperSprite Object Reference"))
  (set `self.Game Over Screens` (`|MakeArray` "/Game/Sprites/28_Sprite.28_Sprite" "/Game/Sprites/27_Sprite.27_Sprite" "/Game/Sprites/26_Sprite.26_Sprite" "/Game/Sprites/25_Sprite.25_Sprite" :!type "PaperSprite Object Reference")))

(event `Game Start`
  (`PaperSpriteComponent.SetSprite` (`self.RenderComponent`) "/Game/Sprites/8_Sprite.8_Sprite")
  (`KismetSystemLibrary.Delay` 0.1)
  (`PaperSpriteComponent.SetSprite` "/Game/Sprites/9_Sprite.9_Sprite")
  (`KismetSystemLibrary.Delay` 0.1))

(event `Ready Screen`
  (`/Game/Blueprints/BP_Pattern.Show Ready Screen` (`self.Pattern Screen`))
  (`PaperSpriteComponent.SetSprite` "/Game/Sprites/1_Sprite.1_Sprite")
  (`KismetSystemLibrary.Delay` 0.1)
  (`PaperSpriteComponent.SetSprite` "/Game/Sprites/2_Sprite.2_Sprite")
  (`KismetSystemLibrary.Delay` 0.1)
  (`PaperSpriteComponent.SetSprite` "/Game/Sprites/3_Sprite.3_Sprite")
  (`KismetSystemLibrary.Delay` 0.1)
  (`PaperSpriteComponent.SetSprite` "/Game/Sprites/7_Sprite.7_Sprite"))

(event `Show Player Press`
  (params (`Player Index` :type Integer :default 0))
  ;[1 1 1] Light Up Spot
  (bind _asbp_game_mode (cast `/Game/Blueprints/BP_GameMode` (`GameplayStatics.GetGameMode`)))
  (`self.Set Background Sprite` (`KismetArrayLibrary.Array_Get` (`self.Player Screens`) `Player Index`))
  (`KismetSystemLibrary.RetriggerableDelay` 0.5)
  (if (`/Game/Blueprints/BP_GameMode.Round Started` _asbp_game_mode)
    (`PaperSpriteComponent.SetSprite` (`self.RenderComponent`) "/Game/Sprites/7_Sprite.7_Sprite")))

(event `Show Player`
  (params (`Player Index` :type Integer :default 0))
  (`PaperSpriteComponent.SetSprite` (`KismetArrayLibrary.Array_Get` (`self.Player Screens`) `Player Index`)))

(event `Idle Screen`
  (`PaperSpriteComponent.SetSprite` "/Game/Sprites/7_Sprite.7_Sprite"))

(event `Show Player Game Over`
  (params (`Player Index` :type Integer :default 0))
  (`PaperSpriteComponent.SetSprite` (`KismetArrayLibrary.Array_Get` (`self.Game Over Screens`) `Player Index`)))

(event `Timer Over`
  (`PaperSpriteComponent.SetSprite` "/Game/Sprites/29_Sprite.29_Sprite"))

(fn `UserConstructionScript`)