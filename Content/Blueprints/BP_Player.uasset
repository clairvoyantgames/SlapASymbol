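; BP_Player handles the player's item placement input and relays it to BP_GameMode.
; PlaceItem acts on game state: it starts the game, sets up a round or changes mode once the intro completes, or places an item mid-round.
; Placement allows one use per input index within the current level, flagging PlacedItems before calling TryUsingItem.
; ClearArrays empties PlayerRoundItems and resets those flags.
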(event `self.ReceiveBeginPlay`
  ;[1 1 1] Init
  (bind _asbp_game_mode (cast `/Game/Blueprints/BP_GameMode` (`GameplayStatics.GetGameMode`)))
  (set `self.Game Mode` _asbp_game_mode))

(event `Place Item`
  (params (`Player Input Index` :type Integer))
  (bind _game_mode (`self.Game Mode`))
  (bind _game_mode_2 (`self.Game Mode`))
  (bind _intro_complete (`/Game/Blueprints/BP_GameMode.Intro Complete` _game_mode_2))
  ;[1 1 1] Placement Logic
  (set `self.Player Input Index` `Player Input Index`)
  (if (`/Game/Blueprints/BP_GameMode.Game Started` _game_mode)
    (if (`/Game/Blueprints/BP_GameMode.Round Started` _game_mode)
      (if (and (`/Game/Blueprints/BP_GameMode.Round Started` _game_mode) (<= (`self.Player Input Index`) (- (`/Game/Blueprints/BP_GameMode.Current Level` _game_mode) 1)) (not (`|GetArrayItem` (`self.Placed Items`) (`self.Player Input Index`))))
        ;[1 1 1] Check for place
        (`KismetArrayLibrary.Array_Set` (`self.Placed Items`) (`self.Player Input Index`) true true)
        (`/Game/Blueprints/BP_GameMode.Try Using Item` (`self.Game Mode`) self))
      (elif (== (`self.Player Input Index`) 0)
        (if _intro_complete
          (`/Game/Blueprints/BP_GameMode.Setup Round` (`self.Game Mode`)))
        (elif _intro_complete
          (`/Game/Blueprints/BP_GameMode.Change Mode` _game_mode_2 (== (`self.Player Input Index`) 1)))))
    (else
      (`/Game/Blueprints/BP_GameMode.Start Game` (`self.Game Mode`)))))

(event `Clear Arrays`
  (bind _placed_items (`self.Placed Items`))
  ;[1 1 1] Clear Items
  (`KismetArrayLibrary.Array_Clear` (`self.Player Round Items`))
  (for (_ _array_index) _placed_items
    (`KismetArrayLibrary.Array_Set` _placed_items _array_index false true)))

(fn `UserConstructionScript`)