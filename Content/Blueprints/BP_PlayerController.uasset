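; Player controller that handles item-placement input for four players, each with three item actions.
; Each input action passes an item index and player index to a shared PlaceItem event, which looks up that player in BP_GameMode's Players array and calls its PlaceItem.
; Hardcoded keys also quit the game or trigger a custom event on the game mode.
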(event `Key|C`
  ;[1 1 1] Quit Game
  (:`Pressed`
    (`KismetSystemLibrary.QuitGame` null "Quit")))

(event `Key|NumPadZero`
  (:`Pressed`
    (bind _asbp_game_mode (cast `/Game/Blueprints/BP_GameMode` (`GameplayStatics.GetGameMode`)))
    (`/Game/Blueprints/BP_GameMode.CustomEvent_0` _asbp_game_mode)))

(event `InputAction|P1 Item 1`
  ;[1 1 1] Item Placing
  (:`Pressed`
    (`self.Place Item` (`self.Item 1 Index`) (`self.Player 1 Index`))))

(event `InputAction|P2 Item 1`
  ;[1 1 1] Item Placing
  (:`Pressed`
    (`self.Place Item` (`self.Item 1 Index`) (`self.Player 2 Index`))))

(event `InputAction|P3 Item 1`
  ;[1 1 1] Item Placing
  (:`Pressed`
    (`self.Place Item` (`self.Item 1 Index`) (`self.Player 3 Index`))))

(event `InputAction|P4 Item 1`
  ;[1 1 1] Item Placing
  (:`Pressed`
    (`self.Place Item` (`self.Item 1 Index`) (`self.Player 4 Index`))))

(event `InputAction|P1 Item 2`
  ;[1 1 1] Item Placing
  (:`Pressed`
    (`self.Place Item` (`self.Item 2 Index`) (`self.Player 1 Index`))))

(event `InputAction|P2 Item 2`
  ;[1 1 1] Item Placing
  (:`Pressed`
    (`self.Place Item` (`self.Item 2 Index`) (`self.Player 2 Index`))))

(event `InputAction|P3 Item 2`
  ;[1 1 1] Item Placing
  (:`Pressed`
    (`self.Place Item` (`self.Item 2 Index`) (`self.Player 3 Index`))))

(event `InputAction|P4 Item 2`
  ;[1 1 1] Item Placing
  (:`Pressed`
    (`self.Place Item` (`self.Item 2 Index`) (`self.Player 4 Index`))))

(event `InputAction|P1 Item 3`
  ;[1 1 1] Item Placing
  (:`Pressed`
    (`self.Place Item` (`self.Item 3 Index`) (`self.Player 1 Index`))))

(event `InputAction|P2 Item 3`
  ;[1 1 1] Item Placing
  (:`Pressed`
    (`self.Place Item` (`self.Item 3 Index`) (`self.Player 2 Index`))))

(event `InputAction|P3 Item 3`
  ;[1 1 1] Item Placing
  (:`Pressed`
    (`self.Place Item` (`self.Item 3 Index`) (`self.Player 3 Index`))))

(event `InputAction|P4 Item 3`
  ;[1 1 1] Item Placing
  (:`Pressed`
    (`self.Place Item` (`self.Item 3 Index`) (`self.Player 4 Index`))))

(event `Place Item`
  (params (`Item Index` :type Integer :default 0) (`Player Index` :type Integer :default 0))
  ;[1 1 1] Place Item
  (bind _asbp_game_mode (cast `/Game/Blueprints/BP_GameMode` (`GameplayStatics.GetGameMode`)))
  (`/Game/Blueprints/BP_Player.Place Item` (`KismetArrayLibrary.Array_Get` (`/Game/Blueprints/BP_GameMode.Players` _asbp_game_mode) `Player Index`) `Item Index`))

(fn `UserConstructionScript`)