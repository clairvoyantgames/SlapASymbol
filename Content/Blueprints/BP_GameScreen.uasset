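; Game screen for a shape memory game, displaying logo, mode choice, ready, memorize and game-over sprites, plus a player spot indicator.
; BeginPlay builds sprite arrays, and events swap sprites by index.
; SetPattern shuffles the shapes and flashes a level-scaled count through a delayed recursive event, then calls ShowPlayerItems on BP_GameMode.
; ShowEachItem similarly steps through given item indices, which refer to the shuffled shape order.
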(event `self.ReceiveBeginPlay`
  ;[1 1 1] Init Sprite Arrays
  (set `self.Spots` (`|MakeArray` "/Game/Sprites/spot1_Sprite.spot1_Sprite" "/Game/Sprites/spot2_Sprite.spot2_Sprite" "/Game/Sprites/spot3_Sprite.spot3_Sprite" "/Game/Sprites/spot4_Sprite.spot4_Sprite" :!type "PaperSprite Object Reference"))
  (set `self.Shapes` (`|MakeArray` "/Game/Sprites/s_bone_Sprite.s_bone_Sprite" "/Game/Sprites/s_circle_Sprite.s_circle_Sprite" "/Game/Sprites/s_diamond_Sprite.s_diamond_Sprite" "/Game/Sprites/s_fish_Sprite.s_fish_Sprite" "/Game/Sprites/s_heart_Sprite.s_heart_Sprite" "/Game/Sprites/s_moon_Sprite.s_moon_Sprite" "/Game/Sprites/s_pac_Sprite.s_pac_Sprite" "/Game/Sprites/s_spade_Sprite.s_spade_Sprite" "/Game/Sprites/s_square_Sprite.s_square_Sprite" "/Game/Sprites/s_star_Sprite.s_star_Sprite" "/Game/Sprites/s_triangle_Sprite.s_triangle_Sprite" "/Game/Sprites/s_x_Sprite.s_x_Sprite" :!type "PaperSprite Object Reference"))
  (set `self.Modes` (`|MakeArray` "/Game/Sprites/choose_game1_Sprite.choose_game1_Sprite" "/Game/Sprites/choose_game2_Sprite.choose_game2_Sprite" :!type "PaperSprite Object Reference")))

(event `Show Spot By Player Index`
  (params (`Player Index` :type Integer :default 0))
  ;[1 1 1] Show Spot By Player Index
  (`PaperSpriteComponent.SetSprite` (`self.Spot`) (`KismetArrayLibrary.Array_Get` (`self.Spots`) `Player Index`)))

(event `Clear Spot`
  ;[1 1 1] Clear Spot
  (`PaperSpriteComponent.SetSprite` (`self.Spot`) null))

(event `Show Item`
  (params (`Item Index` :type Integer :default 0))
  ;[1 1 1] Show Items by Index
  (`PaperSpriteComponent.SetSprite` (`self.Screen`) (`KismetArrayLibrary.Array_Get` (`self.Shapes`) `Item Index`)))

(event `Show Each Item`
  (params (Items :type "Array of Integer") (Index :type Integer :default 0))
  ;[1 1 1] Show Each Player Item by Item Index
  (if (!= (`KismetArrayLibrary.Array_Length` Items) Index)
    (`PaperSpriteComponent.SetSprite` (`self.Screen`) (`KismetArrayLibrary.Array_Get` (`self.Shapes`) (`KismetArrayLibrary.Array_Get` Items Index)))
    (`KismetSystemLibrary.Delay` 0.5)
    (`self.Show Each Item` Items (+ Index 1))))

(event `Show Memorize Screen`
  ;[1 1 1] Show Memorize
  (`PaperSpriteComponent.SetSprite` (`self.Screen`) "/Game/Sprites/memorize_Sprite.memorize_Sprite"))

(event `Show Game Mode`
  (params (`Mode Index` :type Integer :default 0))
  ;[1 1 1] Game Mode
  (`PaperSpriteComponent.SetSprite` (`KismetArrayLibrary.Array_Get` (`self.Modes`) `Mode Index`)))

(event `Set Pattern`
  (params (`Current Level` :type Integer :default 0))
  ;[1 1 1] Set Pattern
  (`KismetArrayLibrary.Array_Shuffle` (`self.Shapes`))
  (`self.Set All Sprites` 0 (* `Current Level` 3)))

(event `Show Logo Screen`
  ;[1 1 1] Show Logo
  (`PaperSpriteComponent.SetSprite` (`self.Screen`) "/Game/Sprites/logo_Sprite.logo_Sprite"))

(event `Show Ready Screen`
  ;[1 1 1] Show Ready
  (`PaperSpriteComponent.SetSprite` (`self.Screen`) "/Game/Sprites/ready_Sprite.ready_Sprite"))

(event `Clear Screen`
  ;[1 1 1] Clear Screen
  (`PaperSpriteComponent.SetSprite` (`self.Screen`) null))

(event `Show Game Over Screen`
  ;[1 1 1] Show Game Over
  (`PaperSpriteComponent.SetSprite` (`self.Screen`) "/Game/Sprites/s_invader_Sprite.s_invader_Sprite"))

(event `Set All Sprites`
  (params (Index :type Integer :default 0) (Total :type Integer :default 0))
  ;[1 1 1] Show Pattern
  (if (< Index Total)
    (`PaperSpriteComponent.SetSprite` (`self.Screen`) (`KismetArrayLibrary.Array_Get` (`self.Shapes`) Index))
    (`KismetSystemLibrary.Delay` 1.0)
    (`PaperSpriteComponent.SetSprite` (`self.Screen`) null)
    (`self.Set All Sprites` (+ Index 1) Total)
    (else
      (bind _asbp_game_mode (cast `/Game/Blueprints/BP_GameMode` (`GameplayStatics.GetGameMode`)))
      (`/Game/Blueprints/BP_GameMode.Show Player Items` _asbp_game_mode))))

(fn `UserConstructionScript`)