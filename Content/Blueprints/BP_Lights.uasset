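; BP_Lights is a sprite-based screen light display that shows game states: idle, start, ready, current player, and game over by player or timer.
; Each event swaps the RenderComponent sprite, using per-player sprite arrays filled on BeginPlay for player and game-over screens.
; Start and ready animations chain Delays, while game-over events re-call themselves via LoopCounter to flash three times before switching the lights off.
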(event `Set Background Sprite`
  (params (Sprite :type "PaperSprite Object Reference"))
  ;[1 1 1] Set Background
  (`PaperSpriteComponent.SetSprite` (`self.RenderComponent`) Sprite))

(event `self.ReceiveBeginPlay`
  ;[1 1 1] Init Objects and Sprite Arrays
  (set `self.Player Screens` (`|MakeArray` "/Game/Sprites/14_Sprite.14_Sprite" "/Game/Sprites/6_Sprite.6_Sprite" "/Game/Sprites/5_Sprite.5_Sprite" "/Game/Sprites/4_Sprite.4_Sprite" :!type "PaperSprite Object Reference"))
  (set `self.Game Over Screens` (`|MakeArray` "/Game/Sprites/28_Sprite.28_Sprite" "/Game/Sprites/27_Sprite.27_Sprite" "/Game/Sprites/26_Sprite.26_Sprite" "/Game/Sprites/25_Sprite.25_Sprite" :!type "PaperSprite Object Reference")))

(event `Set Screen Lights Off`
  ;[1 1 1] Turn Off Screen Lights
  (`self.Set Background Sprite` "/Game/Sprites/0_Sprite.0_Sprite"))

(event `Idle Screen`
  ;[1 1 1] Idle
  (`PaperSpriteComponent.SetSprite` (`self.RenderComponent`) "/Game/Sprites/7_Sprite.7_Sprite"))

(event `Game Start`
  ;[1 1 1] Game Start
  (`PaperSpriteComponent.SetSprite` (`self.RenderComponent`) "/Game/Sprites/7_Sprite.7_Sprite")
  (`KismetSystemLibrary.Delay` 0.2)
  (`PaperSpriteComponent.SetSprite` (`self.RenderComponent`) "/Game/Sprites/3_Sprite.3_Sprite")
  (`KismetSystemLibrary.Delay` 0.2)
  (`PaperSpriteComponent.SetSprite` (`self.RenderComponent`) "/Game/Sprites/7_Sprite.7_Sprite")
  (`KismetSystemLibrary.Delay` 0.2)
  (`PaperSpriteComponent.SetSprite` (`self.RenderComponent`) "/Game/Sprites/3_Sprite.3_Sprite")
  (`KismetSystemLibrary.Delay` 0.2)
  (`PaperSpriteComponent.SetSprite` (`self.RenderComponent`) "/Game/Sprites/7_Sprite.7_Sprite")
  (`KismetSystemLibrary.Delay` 0.2)
  (`PaperSpriteComponent.SetSprite` (`self.RenderComponent`) "/Game/Sprites/3_Sprite.3_Sprite")
  (`KismetSystemLibrary.Delay` 0.2)
  (`PaperSpriteComponent.SetSprite` (`self.RenderComponent`) "/Game/Sprites/7_Sprite.7_Sprite")
  (`KismetSystemLibrary.Delay` 0.2)
  (`self.Idle Screen`))

(event `Ready Screen`
  ;[1 1 1] Ready
  (`PaperSpriteComponent.SetSprite` (`self.RenderComponent`) "/Game/Sprites/1_Sprite.1_Sprite")
  (`KismetSystemLibrary.Delay` 0.1)
  (`PaperSpriteComponent.SetSprite` (`self.RenderComponent`) "/Game/Sprites/2_Sprite.2_Sprite")
  (`KismetSystemLibrary.Delay` 0.1)
  (`PaperSpriteComponent.SetSprite` (`self.RenderComponent`) "/Game/Sprites/3_Sprite.3_Sprite")
  (`KismetSystemLibrary.Delay` 0.1)
  (`self.Idle Screen`))

(event `Show Player`
  (params (`Player Index` :type Integer :default 0))
  ;[1 1 1] Player
  (`PaperSpriteComponent.SetSprite` (`self.RenderComponent`) (`KismetArrayLibrary.Array_Get` (`self.Player Screens`) `Player Index`)))

(event `Show Player Game Over`
  (params (`Player Index` :type Integer :default 0))
  (bind _loop_counter (`self.Loop Counter`))
  ;[1 1 1] Player Game Over
  (`PaperSpriteComponent.SetSprite` (`self.RenderComponent`) (`KismetArrayLibrary.Array_Get` (`self.Game Over Screens`) `Player Index`))
  (`KismetSystemLibrary.Delay` 0.2)
  (`self.Game Over Screen`)
  (`KismetSystemLibrary.Delay` 0.2)
  (if (== _loop_counter 2)
    (set `self.Loop Counter` 0)
    (`self.Set Screen Lights Off`)
    (else
      (set `self.Loop Counter` (+ _loop_counter 1))
      (`self.Show Player Game Over` `Player Index`))))

(event `Timer Over`
  (bind _loop_counter (`self.Loop Counter`))
  ;[1 1 1] Time Game Over
  (`PaperSpriteComponent.SetSprite` (`self.RenderComponent`) "/Game/Sprites/29_Sprite.29_Sprite")
  (`KismetSystemLibrary.Delay` 0.2)
  (`self.Game Over Screen`)
  (`KismetSystemLibrary.Delay` 0.2)
  (if (== _loop_counter 2)
    (set `self.Loop Counter` 0)
    (`self.Set Screen Lights Off`)
    (else
      (set `self.Loop Counter` (+ _loop_counter 1))
      (`self.Timer Over`))))

(event `Game Over Screen`
  ;[1 1 1] Game Over Idle
  (`self.Set Background Sprite` "/Game/Sprites/24_Sprite.24_Sprite"))

(fn `UserConstructionScript`)